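; Game mode for Project Cleaver that manages checkpoint respawning and the pause menu.
; On begin play it finds the checkpoint flagged as the beginning, printing errors if none or several are set, and caches the player character.
; Respawn destroys that character, spawns and possesses a new one at the last checkpoint, then calls OnRespawn.
; A pause toggle creates or removes the menu widget, switching game pause, cursor and input mode.
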(event Custom|SetLastCheckpoint
  (params (ThisCheckpoint :type BP%20Check%20Point%20Object%20Reference))
  ;[1 1 1] Set last checkpoint
  (Variables|Default|SetLastCheckpoint ThisCheckpoint))

(event Custom|DoRespawn
  ;[1 1 1] Remove and Create new player instance
  (CallFunction|RemoveCurrentPlayer)
  (CallFunction|SpawnNewPlayer)
  (Default|CallOnRespawn (Variables|Default|GetCurrentPlayer)))

(event EventRespawn
  ;[1 1 1] Remove and Create new player instance
  (CallFunction|RemoveCurrentPlayer)
  (CallFunction|SpawnNewPlayer)
  (Default|CallOnRespawn (Variables|Default|GetCurrentPlayer)))

(event EventBeginPlay
  ;[1 1 1] (begin) Get begin checkpoint and set current player
  (Utilities|FlowControl|Sequence
    (:then_0
      (CallFunction|FetchBeginCheckpoint))
    (:then_1
      (Variables|Default|SetCurrentPlayer (Game|GetPlayerCharacter 0)))))

(event EventChangePauseMenuState
  (if (Variables|Default|GetbIsPauseMenuOpen)
    (CallFunction|ClosePauseMenu)
    (else
      (CallFunction|OpenPauseMenu))))

(fn ConstructionScript)

(fn RemoveCurrentPlayer
  (Actor|DestroyActor (Variables|Default|GetCurrentPlayer)))

(fn SpawnNewPlayer
  (bind _returnvalue (Game|SpawnActorfromClass "/Game/FirstPerson/Blueprints/BP_FirstPersonCharacter.BP_FirstPersonCharacter_C" (Transformation|GetActorTransform (Variables|Default|GetLastCheckpoint)) "AdjustIfPossibleButAlwaysSpawn" "MultiplyWithRoot" 0 0))
  (bind _output_get (Variables|Default|SetCurrentPlayer _returnvalue))
  (bind _aspawn (Utilities|Casting|CastToPawn _output_get))
  (Pawn|Possess (Game|GetPlayerController 0) _aspawn))

(fn FetchBeginCheckpoint
  (bind _outactors (Actor|GetAllActorsOfClass "/Game/ProjectCleaver/Core/RespawnSystem/BP_CheckPoint.BP_CheckPoint_C"))
  (for _array_element _outactors
    (if (Variables|/Game/ProjectCleaver/Core/RespawnSystem/BP_CheckPoint.BP_CheckPoint_C|GetIsBeginCheckpoint _array_element)
      (Utilities|Array|Add (LocalVariables|GetBeginCheckpoints) _array_element)
      (Variables|Default|SetLastCheckpoint _array_element)))
  (Utilities|IsValid (Variables|Default|GetLastCheckpoint)
    (:Is%20Valid
      ;[1 1 1] Check if there is more than one begin checkpoint and log them.
      (if (> (Utilities|Array|Length (LocalVariables|GetBeginCheckpoints)) 1)
        (for _array_element_2 (LocalVariables|GetBeginCheckpoints)
          (bind _output_get (LocalVariables|SetObjectNames (Utilities|String|Append (LocalVariables|GetObjectNames) " : " (Utilities|GetDisplayName _array_element_2)))))
        (Development|PrintString (Utilities|String|Append "TOO MANY Begin Checkpoints, set only one checkpoint as beginning!!!" "All checkpoints are:" _output_get) true true "(R=1.000000,G=0.000000,B=0.016654,A=1.000000)" 1e+01)))
    (:Is%20Not%20Valid
      (Development|PrintString "NO Begin Checkpoint SET !!!!" true true "(R=1.000000,G=0.000000,B=0.031044,A=1.000000)" 1e+01))))

(fn ClosePauseMenu
  (bind _returnvalue (Game|GetPlayerController 0))
  (Input|SetInputModeGameOnly _returnvalue false)
  (bind _output_get (Variables|Default|SetbIsPauseMenuOpen false))
  (bind _output_get_2 (Variables|/Script/Engine.PlayerController|SetbShowMouseCursor _returnvalue _output_get))
  (Game|SetGamePaused _output_get_2)
  (Widget|RemovefromParent (Variables|Default|GetPauseMenuWidget)))

(fn OpenPauseMenu
  (bind _returnvalue (Game|GetPlayerController 0))
  (bind _returnvalue_2 (UserInterface|CreateWidget "/Game/ProjectCleaver/UI/WBP_PauseMenu.WBP_PauseMenu_C" _returnvalue))
  (bind _output_get (Variables|Default|SetPauseMenuWidget _returnvalue_2))
  (UserInterface|Viewport|AddtoViewport _output_get 0)
  (bind _output_get_2 (Variables|Default|SetbIsPauseMenuOpen true))
  (bind _output_get_3 (Variables|/Script/Engine.PlayerController|SetbShowMouseCursor _returnvalue _output_get_2))
  (Game|SetGamePaused _output_get_3)
  (Input|SetInputModeGameandUI _returnvalue _returnvalue_2 "DoNotLock" true false)
  (return))

(fn GetRespawnEvent
  (return 0))