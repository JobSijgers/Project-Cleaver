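; BP_CheckPoint is a checkpoint actor that records itself as the player's latest respawn point when touched.
; When the player character overlaps its Box, it passes itself to BP_PCGameModeBase through SetLastCheckpoint.
; The first time this happens it also sends the player a very large heal via HealMessage, then clears CanHeal so later visits only update the checkpoint.
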(event OnComponentBeginOverlap(Box)
  (params (OverlappedComponent :type Primitive%20Component%20Object%20Reference) (OtherActor :type Actor%20Object%20Reference) (OtherComp :type Primitive%20Component%20Object%20Reference) (OtherBodyIndex :type Integer) (bFromSweep :type Boolean) (SweepResult :type Hit%20Result%20Structure%20%28by%20ref%29))
  (bind _returnvalue (Game|GetPlayerCharacter 0))
  ;[1 1 1] Set new last checkpoint in gamemode when collide with player and heal at first interaction
  (if (== OtherActor _returnvalue)
    (bind _asbp_pcgame_mode_base (Utilities|Casting|CastToBP_PCGameModeBase (Game|GetGameMode)))
    (Default|SetLastCheckpoint _asbp_pcgame_mode_base self)
    (if (Variables|Default|GetCanHeal)
      (Class|BPIHealable|Heal(Message) _returnvalue 1000000)
      (Variables|Default|SetCanHeal false))))

(fn ConstructionScript)