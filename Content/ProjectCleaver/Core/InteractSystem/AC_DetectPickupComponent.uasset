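; Actor component that detects and highlights pickups in the world with a line trace from a supplied start and direction.
; DetectPickup stores a hit actor implementing BPI_Pickups as PotentialPickup and enables custom depth on all its primitive components.
; The highlight clears only when the trace hits nothing, not when it moves onto another actor.
; Pickup is a stub that always reports IsWeapon as false.
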(event Custom|DetectPickup
  (params (StartPosLineTrace :type Vector) (TraceDirection :type Vector))
  ;[1 1 1] Draws Line to look for pickups
  (bind (_outhit _returnvalue) (Collision|LineTraceForObjects StartPosLineTrace (+ StartPosLineTrace (* TraceDirection (Variables|Default|GetDetectionTraceLength))) (Utilities|Array|MakeArray "ObjectTypeQuery1" "ObjectTypeQuery2") false 0 "None"))
  (if _returnvalue
    (if (Utilities|DoesObjectImplementInterface (.HitActor (Collision|BreakHitResult _outhit)) "/Game/ProjectCleaver/Core/InteractSystem/BPI_Pickups.BPI_Pickups_C")
      (Utilities|IsValid (Variables|Default|GetPotentialPickup)
        (:Is%20Valid
          (if (not (== (Variables|Default|GetPotentialPickup) (.HitActor (Collision|BreakHitResult _outhit))))
            (CallFunction|ChangeHighlightState true (.HitActor (Collision|BreakHitResult _outhit)) :!label _label)
            (Variables|Default|SetPotentialPickup (.HitActor (Collision|BreakHitResult _outhit)))))
        (:Is%20Not%20Valid
          (goto _label))))
    (else
      (Utilities|IsValid (Variables|Default|GetPotentialPickup)
        (:Is%20Valid
          (CallFunction|ChangeHighlightState false (Variables|Default|GetPotentialPickup))
          (Variables|Default|SetPotentialPickup 0))))))

(fn ChangeHighlightState
  (params (State :type Boolean) (ActorToChange :type Actor%20Object%20Reference))
  (Utilities|IsValid ActorToChange
    (:Is%20Valid
      (for _array_element (Actor|GetComponentsByClass ActorToChange "/Script/Engine.PrimitiveComponent")
        (Rendering|SetRenderCustomDepth _array_element State))
      (return))))

(fn Pickup
  (return 0 false))