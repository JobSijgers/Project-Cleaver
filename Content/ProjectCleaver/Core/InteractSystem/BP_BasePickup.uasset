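; Base pickup actor for the interact system, representing an item described by a data asset.
; The construction script copies the asset's weapon mesh and its first material onto the EmptyFrame component.
; Pickup plays a sound at its location, destroys the actor, fires OnPickup, and returns the item data with a weapon flag.
; SendMessageToGate is an empty stub.
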(fn ConstructionScript
  (bind _obtaindataasset (Variables|Default|GetObtainDataAsset))
  (bind _weaponmesh (Variables|/Game/ProjectCleaver/Core/CombatSystem/WeaponData.WeaponData_C|GetWeaponMesh _obtaindataasset))
  (Utilities|IsValid (Variables|Default|GetObtainDataAsset)
    (:Is%20Valid
      (Components|StaticMesh|SetStaticMesh (Variables|Default|GetEmpty%20Frame) _weaponmesh)
      (Rendering|Material|SetMaterial (Variables|Default|GetEmpty%20Frame) 0 (Rendering|Material|GetMaterial _weaponmesh 0)))))

(fn SendMessagetoGate)

(fn Pickup
  (Audio|SpawnSoundatLocation "/Game/Developers/Pedro/Collections/Audio/Pickup/PickupSound.PickupSound" (Transformation|GetWorldLocation (Variables|Default|GetDefaultSceneRoot)) "0, 0, 0" 1.0 1.0 0.0 0 0)
  (Actor|DestroyActor)
  (Default|CallOnPickup)
  (return (Variables|Default|GetObtainDataAsset) (Variables|Default|GetbIsWeapon)))